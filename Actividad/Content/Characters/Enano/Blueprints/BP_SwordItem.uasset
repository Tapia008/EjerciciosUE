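; Sword weapon actor for the Enano character that damages BP_Enemigo actors on contact.
; A capsule overlap subtracts WeaponDamage directly from the enemy's HP and destroys the enemy when HP reaches zero or below.
; ToggleWeapon switches the capsule collision on or off as the hit window, starting off at BeginPlay.
; Enable and Disable separately show or hide the whole component hierarchy without touching collision.
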(event OnComponentBeginOverlap(Capsule)
  (params (OverlappedComponent :type Primitive%20Component%20Object%20Reference) (OtherActor :type Actor%20Object%20Reference) (OtherComp :type Primitive%20Component%20Object%20Reference) (OtherBodyIndex :type Integer) (bFromSweep :type Boolean) (SweepResult :type Hit%20Result%20Structure%20%28by%20ref%29))
  ;[0.15 0.15 0.15 0.5] Daño del arma
  (bind _asbp_enemigo (Utilities|Casting|CastToBP_Enemigo OtherActor))
  (bind _output_get (Variables|/Game/Characters/Enano/BP_Enemigo.BP_Enemigo_C|SetHP _asbp_enemigo (- (Variables|/Game/Characters/Enano/BP_Enemigo.BP_Enemigo_C|GetHP _asbp_enemigo) (Variables|Default|GetWeapon%20damage))))
  (Math|Float|CompareFloat _output_get 0.0
    (:==
      _)
    (:<
      _))
  (bind _asbp_enemigo_2 (Utilities|Casting|CastToBP_Enemigo OtherActor))
  (Actor|DestroyActor _asbp_enemigo_2))

(event EventBeginPlay
  (CallFunction|ToggleWeapon false))

(fn ConstructionScript)

(fn ToggleWeapon
  (params (Is%20Active :type Boolean))
  (bind _capsule (Variables|Default|GetCapsule))
  (if Is%20Active
    (Collision|SetCollisionEnabled _capsule "QueryAndPhysics")
    (else
      (Collision|SetCollisionEnabled _capsule "NoCollision"))))

(fn Enable
  (Rendering|SetVisibility (Variables|Default|GetDefaultSceneRoot) true true))

(fn Disable
  (Rendering|SetVisibility (Variables|Default|GetDefaultSceneRoot) false true))