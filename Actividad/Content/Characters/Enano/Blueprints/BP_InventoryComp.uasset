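; Inventory component, in the Enano character's folder, that keeps an array of items the owner picks up and drops.
; Grab and drop check each item's IsGraph flag, update the array, and delegate to that item's BPItemComp.
; Drops land in front of the owner, and DropLastItem releases the most recently added item.
; After each change it prints item names and descriptions, or an empty-inventory message, on screen in Spanish.
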(event EventBeginPlay)

(event EventTick
  (params (DeltaSeconds :type Float%20%28single-precision%29)))

(fn GrabItem
  (params (ItemIn :type BP%20Item%20Object%20Reference))
  (bind _bp_itemcomp (Variables|/Game/Characters/Enano/Blueprints/BP_Item.BP_Item_C|GetBP_ItemComp ItemIn))
  (if (not (Variables|/Game/Characters/Enano/Blueprints/BP_ItemComp.BP_ItemComp_C|GetIsGraph _bp_itemcomp))
    (Utilities|Array|Add (Variables|Default|GetItems) ItemIn)
    (Default|Grab _bp_itemcomp)
    (CallFunction|PrintItem)))

(fn DropItem
  (params (ItemOut :type BP%20Item%20Object%20Reference))
  (bind _returnvalue (Components|GetOwner))
  (bind _bp_itemcomp (Variables|/Game/Characters/Enano/Blueprints/BP_Item.BP_Item_C|GetBP_ItemComp ItemOut))
  (if (Variables|/Game/Characters/Enano/Blueprints/BP_ItemComp.BP_ItemComp_C|GetIsGraph _bp_itemcomp)
    (Utilities|Array|RemoveItem (Variables|Default|GetItems) ItemOut)
    (Default|Drop _bp_itemcomp (+ (Transformation|GetActorLocation _returnvalue) (* (Transformation|GetActorForwardVector _returnvalue) 2e+02)))
    (CallFunction|PrintItem)
    (return ItemOut)))

(fn DropLastItem
  (bind _items (Variables|Default|GetItems))
  (bind _returnvalue (Utilities|Array|LastIndex _items))
  (if (Utilities|Array|IsValidIndex _items _returnvalue)
    (CallFunction|DropItem (Utilities|Array|Get(acopy) _items _returnvalue))
    (else
      (Development|PrintString "No hay nada en el inventario"))))

(fn PrintItem
  (if (not (Utilities|Array|IsEmpty (Variables|Default|GetItems)))
    (for _array_element (Variables|Default|GetItems)
      (Development|PrintString (Utilities|String|Append "Objeto: " (Variables|/Game/Characters/Enano/Blueprints/BP_ItemComp.BP_ItemComp_C|GetName (Variables|/Game/Characters/Enano/Blueprints/BP_Item.BP_Item_C|GetBP_ItemComp _array_element)) "Descripción: " (Variables|/Game/Characters/Enano/Blueprints/BP_ItemComp.BP_ItemComp_C|GetDescription (Variables|/Game/Characters/Enano/Blueprints/BP_Item.BP_Item_C|GetBP_ItemComp _array_element))) true true "(R=0.000000,G=0.660000,B=1.000000,A=1.000000)" 5.0))
    (else
      (Development|PrintString "No hya nada en el inventario"))))