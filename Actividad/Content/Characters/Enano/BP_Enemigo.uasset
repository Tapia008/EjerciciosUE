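; BP_Enemigo is an enemy Blueprint with a floating health bar that appears only when the player is near.
; Every tick it sets the Healthbar widget's percent from HP out of 100 and rotates the widget component to face the player camera.
; The bar starts hidden, and the Sphere overlap events show or hide it when a BP_ThirdPersonCharacter enters or leaves.
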(event OnComponentBeginOverlap(Sphere)
  (params (OverlappedComponent :type Primitive%20Component%20Object%20Reference) (OtherActor :type Actor%20Object%20Reference) (OtherComp :type Primitive%20Component%20Object%20Reference) (OtherBodyIndex :type Integer) (bFromSweep :type Boolean) (SweepResult :type Hit%20Result%20Structure%20%28by%20ref%29))
  (Utilities|Casting|CastToBP_ThirdPersonCharacter OtherActor)
  (Rendering|SetVisibility (Variables|Default|GetHealthbar) true false))

(event OnComponentEndOverlap(Sphere)
  (params (OverlappedComponent :type Primitive%20Component%20Object%20Reference) (OtherActor :type Actor%20Object%20Reference) (OtherComp :type Primitive%20Component%20Object%20Reference) (OtherBodyIndex :type Integer))
  (Utilities|Casting|CastToBP_ThirdPersonCharacter OtherActor)
  (Rendering|SetVisibility (Variables|Default|GetHealthbar) false false))

(event EventTick
  (params (DeltaSeconds :type Float%20%28single-precision%29))
  ;[0.15 0.15 0.15 0.5] Barra de vida
  (bind _ashealthbar (Utilities|Casting|CastToHealthbar (UserInterface|GetWidget (Variables|Default|GetHealthbar))))
  (Progress|SetPercent (Variables|/Game/Characters/Enano/Healthbar.Healthbar_C|GetHealthbar _ashealthbar) (/ (Variables|Default|GetHP) 1e+02))
  (Transformation|SetWorldRotation (Variables|Default|GetHealthbar) (Math|Rotator|FindLookatRotation (Transformation|GetWorldLocation (Variables|Default|GetHealthbar)) (Transformation|GetWorldLocation (Variables|/Script/Engine.PlayerCameraManager|GetTransformComponent (Game|GetPlayerCameraManager 0)))) false false))

(event EventBeginPlay
  (Rendering|SetVisibility (Variables|Default|GetHealthbar) false false))

(fn ConstructionScript)